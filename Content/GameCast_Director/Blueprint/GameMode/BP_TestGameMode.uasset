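; Test game mode for the GameCast Director that sets up a camera director alongside two local test players.
; On BeginPlay it creates the camera controller widget and binds it to every CameraPreviewActor found in the level.
; It then creates two extra local players and spawns pawns for possession: the director pawn for player 0, first-person and third-person test characters for players 1 and 2.
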(event `self.ReceiveBeginPlay`
  (bind _returnvalue (`GameplayStatics.GetPlayerController` 1))
  (bind _returnvalue_2 (`GameplayStatics.GetPlayerController` 0))
  (bind _returnvalue_3 (`GameplayStatics.GetPlayerController` 2))
  (bind _previewactorsarray (`self.PreviewActorsArray`))
  (`|ExecutionSequence`
    (:`then_0`
      (bind _returnvalue_4 (`|CreateWidget` "/GameCastDirector/UI/WBP_CameraController.WBP_CameraController_C"))
      (bind _output_get (set `self.CameraControlWidget` _returnvalue_4))
      (`UserWidget.AddToViewport` _output_get 0)
      (bind _outactors (`GameplayStatics.GetAllActorsOfClass` "/Script/GameCastDirector.CameraPreviewActor"))
      (for _array_element _outactors
        (`KismetArrayLibrary.Array_Add` _previewactorsarray _array_element))
      (`WBP_CameraPreviewWidget.BindPreviewCameras` (`self.CameraControlWidget`) _previewactorsarray))
    (:`then_1`
      (bind _returnvalue_5 (`GameplayStatics.CreatePlayer` 1))
      (`GameplayStatics.CreatePlayer` 2)
      (`KismetSystemLibrary.PrintString` (`KismetSystemLibrary.GetDisplayName` _returnvalue_5))
      (bind _returnvalue_6 (`|SpawnActorFromClass` "/Game/GameCast_Director/Blueprint/Characters/BP_FirstPersonCharacterTest.BP_FirstPersonCharacterTest_C" (`KismetMathLibrary.MakeTransform` (0.0 0.0 500.0)) "Undefined" "MultiplyWithRoot" _returnvalue null))
      (`Controller.Possess` _returnvalue _returnvalue_6)
      (bind _returnvalue_7 (`|SpawnActorFromClass` "/Game/GameCast_Director/Blueprint/Characters/BP_ThirdPersonTestChar.BP_ThirdPersonTestChar_C" (`KismetMathLibrary.MakeTransform` (0.0 0.0 500.0)) "Undefined" "MultiplyWithRoot" _returnvalue_3 null))
      (`Controller.Possess` _returnvalue_3 _returnvalue_7)
      (bind _returnvalue_8 (`|SpawnActorFromClass` "/GameCastDirector/Blueprints/BP_CameraDirectorPawn.BP_CameraDirectorPawn_C" (`KismetMathLibrary.MakeTransform` (0.0 0.0 500.0)) "Undefined" "MultiplyWithRoot" _returnvalue_2 null))
      (`Controller.Possess` _returnvalue_2 _returnvalue_8))))

(fn `UserConstructionScript`)